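; BP_Projectile is a projectile that moves the player to where it lands or sends them through a portal it hits.
; It caches the player character on BeginPlay and handles hits on its sphere component.
; Hitting a Portal-tagged platform passes that platform's destination and fade colour to the player's TravelThroughPortal.
; Other hits, except on the player, pass impact point and normal to TeleportToProjectile; either teleport destroys the projectile.
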(event OnComponentHit(Sphere)
  (params (HitComponent :type Primitive%20Component%20Object%20Reference) (OtherActor :type Actor%20Object%20Reference) (OtherComp :type Primitive%20Component%20Object%20Reference) (NormalImpulse :type Vector :default "0, 0, 0") (Hit :type Hit%20Result%20Structure%20%28by%20ref%29))
  (bind (_bblockinghit _binitialoverlap _time _distance _location _impactpoint _normal _impactnormal _physmat _hitactor) (Collision|BreakHitResult Hit))
  (if (Actor|ActorHasTag OtherActor "Portal")
    ;[0.333 0.9801 1] Trigger Portal
    (bind _asbp_portal_platform (Utilities|Casting|CastToBP_PortalPlatform OtherActor))
    (Default|TravelThroughPortal (Variables|Default|GetPlayer) (Variables|/Game/Platforms/BP_PortalPlatform.BP_PortalPlatform_C|GetNew%20Location _asbp_portal_platform) (Variables|/Game/Platforms/BP_PortalPlatform.BP_PortalPlatform_C|GetPortal%20Colour _asbp_portal_platform))
    (Actor|DestroyActor)
    (else
      ;[1 0.1427 0.7599] Teleport Player to location
      (Variables|Default|SetHitPos _impactpoint)
      (if (not (Actor|ActorHasTag _hitactor "Player"))
        (Default|TeleporttoProjectile (Variables|Default|GetPlayer) (Variables|Default|GetHitPos) _normal)
        (Actor|DestroyActor)))))

(event EventBeginPlay
  (bind _asbp_third_person_character (Utilities|Casting|CastToBP_ThirdPersonCharacter (Game|GetPlayerCharacter 0)))
  (Variables|Default|SetPlayer _asbp_third_person_character))

(fn ConstructionScript)