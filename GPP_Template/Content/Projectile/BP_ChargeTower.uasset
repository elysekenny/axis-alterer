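; BP_ChargeTower is a pickup station that refills the third-person character's projectiles when it enters the Collider.
; Its Cube bobs on Z around its starting location and oscillates in rotation, both driven every Tick by sine waves of time since creation.
; Overlap begin casts to BP_ThirdPersonCharacter, stores it as Player and calls RefillProjectiles.
; Overlap end only performs the cast, with no further effect.
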(event OnComponentBeginOverlap(Collider)
  (params (OverlappedComponent :type Primitive%20Component%20Object%20Reference) (OtherActor :type Actor%20Object%20Reference) (OtherComp :type Primitive%20Component%20Object%20Reference) (OtherBodyIndex :type Integer) (bFromSweep :type Boolean) (SweepResult :type Hit%20Result%20Structure%20%28by%20ref%29))
  (bind _asbp_third_person_character (Utilities|Casting|CastToBP_ThirdPersonCharacter OtherActor))
  (Variables|Default|SetPlayer _asbp_third_person_character)
  (Default|RefillProjectiles (Variables|Default|GetPlayer)))

(event OnComponentEndOverlap(Collider)
  (params (OverlappedComponent :type Primitive%20Component%20Object%20Reference) (OtherActor :type Actor%20Object%20Reference) (OtherComp :type Primitive%20Component%20Object%20Reference) (OtherBodyIndex :type Integer))
  (Utilities|Casting|CastToBP_ThirdPersonCharacter OtherActor))

(event EventBeginPlay
  (bind _cube (Variables|Default|GetCube))
  ;[1 1 1] Cube  Bob
  (Variables|Default|SetStart%20Location (Variables|/Script/Engine.SceneComponent|GetRelativeLocation _cube))
  (Variables|Default|SetRelative%20Rotation (Variables|/Script/Engine.SceneComponent|GetRelativeRotation _cube)))

(event EventTick
  (params (DeltaSeconds :type Float%20%28single-precision%29))
  (bind _returnvalue (Actor|GetGameTimeSinceCreation))
  (bind _relative_rotation (Variables|Default|GetRelative%20Rotation))
  (bind _rot_speed (Variables|Default|GetRot%20Speed))
  (bind _cube (Variables|Default|GetCube))
  (bind _start_location (Variables|Default|GetStart%20Location))
  (bind _returnvalue_2 (* _returnvalue _rot_speed))
  (bind _returnvalue_3 (Math|Trig|Sin(Degrees) _returnvalue_2))
  (bind _returnvalue_4 (* _returnvalue_3 1.8e+02))
  ;[1 1 1] Cube  Bob
  (Transformation|SetRelativeLocation _cube (Math|Vector|MakeVector (.x _start_location) (.y _start_location) (+ (.z _start_location) (* (Math|Trig|Sin(Degrees) (* (Actor|GetGameTimeSinceCreation) (Variables|Default|GetBob%20Speed))) (Variables|Default|GetBob%20Distance)))) false false)
  (Transformation|SetRelativeRotation _cube (Math|Rotator|MakeRotator (+ _returnvalue_4 0.0) (+ _returnvalue_4 (.pitch _relative_rotation)) (+ _returnvalue_4 (.yaw _relative_rotation))) false false))

(fn ConstructionScript)